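; Player camera manager for the ARPG that overrides BlueprintUpdateCamera to drive the view through a camera state.
; In Gameplay it follows the playable character's camera component and caches its transform and FOV.
; Frozen holds that cached view, while the transition state linearly interpolates location and rotation to a target over a set duration, keeping FOV, then freezes there.
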(fn `BlueprintUpdateCamera`
  (params (CameraTarget :type "Actor Object Reference"))
  (returns (NewCameraLocation :type "Vector Structure") (NewCameraRotation :type "Rotator Structure") (NewCameraFOV :type "Float (single-precision)") (ReturnValue :type Boolean))
  (bind _lastknowncameratransform_location (`KismetMathLibrary.BreakTransform` (`self.LastKnownCameraTransform`)))
  (bind (_lastknowncameratransform_location_2 _lastknowncameratransform_rotation _lastknowncameratransform_scale) (`KismetMathLibrary.BreakTransform` (`self.LastKnownCameraTransform`)))
  (bind (_lastknowncameratransform_location_3 _lastknowncameratransform_rotation_2) (`KismetMathLibrary.BreakTransform` (`self.LastKnownCameraTransform`)))
  (bind (_lastknowncameratransform_location_4 _lastknowncameratransform_rotation_3) (`KismetMathLibrary.BreakTransform` (`self.LastKnownCameraTransform`)))
  (switch `ECameraState` (`self.CurrentCameraState`)
    (:`Frozen`
      (return _lastknowncameratransform_location_4 _lastknowncameratransform_rotation_3 (`self.LastKnownFoV`) true))
    (:`TransitionTowardsFrozenTarget`
      (if (< (`self.CurrentTransitionDuration`) (`self.CurrentTransitionTotalDuration`))
        (bind _output_get (set `self.CurrentTransitionDuration` (+ (`self.CurrentTransitionDuration`) (`GameplayStatics.GetWorldDeltaSeconds`))))
        (bind _returnvalue (/ _output_get (`self.CurrentTransitionTotalDuration`)))
        (return (`KismetMathLibrary.VLerp` _lastknowncameratransform_location (`self.TransitionTargetLocation`) _returnvalue) (`KismetMathLibrary.RLerp` _lastknowncameratransform_rotation_2 (`self.TransitionTargetRotator`) _returnvalue) (`self.LastKnownFoV`) true)
        (else
          (`self.SetFrozen`)
          (set `self.LastKnownCameraTransform` (`KismetMathLibrary.MakeTransform` (`self.TransitionTargetLocation`) (`self.TransitionTargetRotator`) _lastknowncameratransform_scale))
          (return (`self.TransitionTargetLocation`) (`self.TransitionTargetRotator`) (`self.LastKnownFoV`) true))))
    (:`Gameplay`
      (bind _asbp_playable_character (cast `/Game/Blueprints/Character/playableCharacter/BP_playableCharacter` CameraTarget))
      (bind _camera (`/Game/Blueprints/Character/playableCharacter/BP_playableCharacter.Camera` _asbp_playable_character))
      (bind _output_get_2 (set `self.LastKnownCameraTransform` (`SceneComponent.K2_GetComponentToWorld` _camera)))
      (bind _output_get_3 (set `self.LastKnownFoV` (`CameraComponent.FieldOfView` _camera)))
      (return (.location _output_get_2) (.rotation _output_get_2) _output_get_3 true))))

(fn `UserConstructionScript`)