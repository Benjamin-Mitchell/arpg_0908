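; Core game mode Blueprint that handles the opening of a level, from intro cinematic to gameplay.
; On level begin it plays the Bebemebe intro sequence at the world origin.
; When the intro ends, it spawns players manually, then starts the blackboard on every ArpgAIControlledCharacter in the level.
; A disconnected BP_BabyMaybe spawn node never runs, and BeginPlay and Tick are unused.
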(event `self.LevelBeginBP`
  (`self.BeginIntroCinematic` "/Game/Assets/CamSequences/Bebemebe_Intro_Seq.Bebemebe_Intro_Seq" (`KismetMathLibrary.MakeTransform` (0.0 0.0 0.0))))

(event `self.IntroEnded`
  (`self.SpawnPlayersManually`)
  (bind _outactors (`GameplayStatics.GetAllActorsOfClass` "/Script/arpg_0908.arpgAIControlledCharacter"))
  (for _array_element _outactors
    (`arpgAIControlledCharacter.StartBlackboard` _array_element)))

(fn `UserConstructionScript`
  (`parent.UserConstructionScript`))