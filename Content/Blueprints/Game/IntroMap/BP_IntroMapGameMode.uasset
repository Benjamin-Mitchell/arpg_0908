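; Game mode for the intro map that tracks which players are ready.
; It keeps a list of unique ready player IDs, updated by OnPlayerReadyStateChanged from each character's PlayerState.
; Ready and total player counts are broadcast through BP_IntroMapGameState on BeginPlay, after a short delay on PostLogin, and on ready changes.
; The all-players-ready check exists but triggers nothing yet.
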(event `self.ReceiveBeginPlay`
  (`parent.ReceiveBeginPlay`)
  (bind _asbp_intro_map_game_state (cast `/Game/Blueprints/Game/IntroMap/BP_IntroMapGameState` (`GameplayStatics.GetGameState`))
    (:`then`
      (bind _output_get (set `self.Game State` _asbp_intro_map_game_state))
      (`KismetSystemLibrary.PrintString` "got game state")
      (`/Game/Blueprints/Game/IntroMap/BP_IntroMapGameState.BroadcastPlayerReadyCount` _output_get (`KismetArrayLibrary.Array_Length` (`self.ReadyPlayerIDs`)) 0))
    (:`CastFailed`
      (`KismetSystemLibrary.PrintString` "bogies"))))

(event `self.K2_PostLogin`
  (params (NewPlayer :type "PlayerController Object Reference"))
  (`KismetSystemLibrary.Delay` 0.2)
  (if (`KismetSystemLibrary.IsValid` (`self.Game State`))
    (`/Game/Blueprints/Game/IntroMap/BP_IntroMapGameState.BroadcastPlayerReadyCount` (`self.Game State`) (`KismetArrayLibrary.Array_Length` (`self.ReadyPlayerIDs`)) (`GameplayStatics.GetNumPlayerControllers`))))

(fn `OnPlayerReadyStateChanged`
  (params (PlayerCharacter :type "Actor Object Reference") (Ready :type Boolean))
  (locals (PlayerID :type Integer :default 0))
  (bind _asarpg_character (cast `arpgCharacter` PlayerCharacter))
  (set `local.PlayerID` (`PlayerState.PlayerId` (`Controller.PlayerState` (`Pawn.GetController` _asarpg_character))))
  (if Ready
    (`KismetArrayLibrary.Array_AddUnique` (`self.ReadyPlayerIDs`) (`local.PlayerID`))
    (`/Game/Blueprints/Game/IntroMap/BP_IntroMapGameState.BroadcastPlayerReadyCount` (`self.Game State`) (`KismetArrayLibrary.Array_Length` (`self.ReadyPlayerIDs`)) (`GameplayStatics.GetNumPlayerControllers`))
    ; Check if all players are ready
    (if (== (`KismetArrayLibrary.Array_Length` (`self.ReadyPlayerIDs`)) (`GameplayStatics.GetNumPlayerControllers`))
      _)
    (else
      (`KismetArrayLibrary.Array_RemoveItem` (`self.ReadyPlayerIDs`) (`local.PlayerID`))
      (`/Game/Blueprints/Game/IntroMap/BP_IntroMapGameState.BroadcastPlayerReadyCount` (`self.Game State`) (`KismetArrayLibrary.Array_Length` (`self.ReadyPlayerIDs`)) (`GameplayStatics.GetNumPlayerControllers`)))))

(fn `UserConstructionScript`
  (`parent.UserConstructionScript`))