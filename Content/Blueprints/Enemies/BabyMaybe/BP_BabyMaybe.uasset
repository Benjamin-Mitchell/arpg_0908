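; BP_BabyMaybe is an enemy that alternates between Baby and Maybe forms, with its state exposed through blackboard keys.
; BeginPlay resets those keys and stores the level's single BP_BabyTeddy, printing an error otherwise.
; Tick times the current form against its own duration, then only flags NeedsTransform.
; SetIsMaybe applies a form, resetting the timer and local flag, updating the IsMaybe key and multicasting the head mesh swap.
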(event `self.ReceiveBeginPlay`
  (`parent.ReceiveBeginPlay`)
  (`self.SetIsMaybe` (`self.IsMaybe`))
  (`self.SetBlackboardCustomBool` "BabyCryBegun")
  (`self.SetBlackboardCustomBool` "NeedsTransform")
  (`self.SetBlackboardCustomBool` "BabyReachedTeddy")
  (bind _outactors (`GameplayStatics.GetAllActorsOfClass` "/Game/Blueprints/AbilitySystem/Enemy/AbilityActors/BebeMebe/BP_BabyTeddy.BP_BabyTeddy_C"))
  (if (!= (`KismetArrayLibrary.Array_Length` _outactors) 1)
    (`KismetSystemLibrary.PrintString` "ERROR: Incorrect Number of Baby Teddies in the scene!" true true (struct :`R` 1.0 :`A` 1.0) 15.0)
    (else
      (`self.SetBlackboardCustomObject` "BabyTeddyObject" (`|GetArrayItem` _outactors)))))

(event `self.ReceiveTick`
  (params (DeltaSeconds :type "Float (single-precision)"))
  (`parent.ReceiveTick` DeltaSeconds)
  (if (not (`self.NeedsTransform`))
    (`self.UpdateTickForTransform` DeltaSeconds)))

(event `MulticastSetHeadMesh`
  (params (IsMaybe :type Boolean))
  (if IsMaybe
    (`SkeletalMeshComponent.SetSkeletalMeshAsset` (`self.BaseHeadMesh`) (`self.MaybeHeadSkeletalMeshRef`))
    (else
      (`SkeletalMeshComponent.SetSkeletalMeshAsset` (`self.BaseHeadMesh`) (`self.BabyHeadSkeletalMeshRef`)))))

(fn `SetIsMaybe`
  (params (IsMaybe :type Boolean))
  (set `self.FormDurationSoFar` 0.0)
  (set `self.NeedsTransform` false)
  (bind _output_get (set `self.IsMaybe` IsMaybe))
  (`self.SetBlackboardCustomBool` "IsMaybe" _output_get)
  (`self.MulticastSetHeadMesh` (`self.IsMaybe`)))

(fn `SetNeedsTransform`
  (set `self.NeedsTransform` true)
  (`self.SetBlackboardCustomBool` "NeedsTransform" true))

(fn `UpdateTickForTransform`
  (params (B :type "Float (double-precision)"))
  (set `self.FormDurationSoFar` (+ (`self.FormDurationSoFar`) B))
  (if (`self.IsMaybe`)
    (if (>= (`self.FormDurationSoFar`) (`self.MaybeDuration`))
      (`self.SetNeedsTransform` :!label _label))
    (elif (>= (`self.FormDurationSoFar`) (`self.BabyDuration`))
      (goto _label))))

(fn `UserConstructionScript`
  (`parent.UserConstructionScript`))