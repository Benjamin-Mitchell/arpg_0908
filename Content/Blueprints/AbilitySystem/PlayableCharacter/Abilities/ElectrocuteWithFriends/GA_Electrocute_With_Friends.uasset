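; Co-op gameplay ability that links two channeling casters with an electric beam, damaging enemies between them.
; After the intro montage, it adds a synchronization tag and polls for another tagged caster, then attaches the beam GameplayCue.
; A looping timer line-traces between both chest sockets, applying SetByCaller damage to non-friendly hits until the beam duration ends the ability.
; Input release stops the channeling pose but only prints when no beam has begun.
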(event `self.K2_ActivateAbility`
  (`KismetSystemLibrary.PrintString` "Hello")
  (`AbilityTask_PlayMontageAndWait.CreatePlayMontageAndWaitProxy` "None" "/Game/Assets/Rawb/Anims/AM_Cast_Staff_Overhead_Intro.AM_Cast_Staff_Overhead_Intro"
    (:`then`
      (message `CombatInterface.SetInStaffOverheadChannelingLoop` (`self.GetAvatarActorFromActorInfo`) true))
    (:`OnCompleted`
      (`|ExecutionSequence`
        (:`then_0`
          (`self.AddSynchronizationTagToASC`)
          (bind _asarpg_character_base (cast `arpgCharacterBase` (`self.GetAvatarActorFromActorInfo`)))
          (bind _output_get (set `self.AvatarCharacter` _asarpg_character_base))
          (bind (_asynctaskproxy _datahandle) (`WaitSynchronizeAbility.WaitForCheckPlayersWithTag` _output_get (`self.SynchronizeTag`))
            (:`OnNewCaster`
              (for _array_element (`AbilitySystemBlueprintLibrary.GetActorsFromTargetData` _datahandle)
                (bind _asarpg_character_base_2 (cast `arpgCharacterBase` _array_element))
                (set `self.TargetCharacter` _asarpg_character_base_2)
                (`GameplayCueFunctionLibrary.AddGameplayCueOnActor` (`self.GetAvatarActorFromActorInfo`) (struct :`TagName` "GameplayCue.ElectrocuteWithFriends") (`AbilitySystemBlueprintLibrary.MakeGameplayCueParameters` 0.0 0.0 (struct) (struct) (struct) (struct) (struct) (0.0 0.0 0.0) (0.0 0.0 0.0) null null (`self.GetAvatarActorFromActorInfo`) null 1 1 (`Character.Mesh` _asarpg_character_base_2)))
                (set `self.BeamBegun` true)
                (`AbilityTask_WaitDelay.WaitDelay` (`self.BeamDuration`)
                  (:`then`
                    (`KismetSystemLibrary.K2_SetTimerDelegate` (delegate `RaycastAndDealDamage`) (`self.BeamDeltaTime`) true))
                  (:`OnFinish`
                    (`self.K2_RemoveGameplayCue` (struct :`TagName` "GameplayCue.ElectrocuteWithFriends"))
                    (`self.RemoveSynchronizationTagToASC`)
                    (`self.K2_EndAbility`)))))))
        (:`then_1`
          (`AbilityTask_WaitInputRelease.WaitInputRelease` true
            (:`OnRelease`
              (message `CombatInterface.SetInStaffOverheadChannelingLoop` (`self.GetAvatarActorFromActorInfo`) false)
              (if (not (`self.BeamBegun`))
                (`KismetSystemLibrary.PrintString` "endability on input reslease")))))))))

(event `RaycastAndDealDamage`
  (bind _outhits (`KismetSystemLibrary.LineTraceMultiByProfile` (`SceneComponent.GetSocketLocation` (`Character.Mesh` (`self.AvatarCharacter`)) "ChestSocket") (`SceneComponent.GetSocketLocation` (`Character.Mesh` (`self.TargetCharacter`)) "ChestSocket") "Pawn" false (`|MakeArray` (`self.TargetCharacter`) (`self.AvatarCharacter`) :!type "Actor Object Reference")))
  (for _array_element _outhits
    (bind (_bblockinghit _binitialoverlap _time _distance _location _impactpoint _normal _impactnormal _physmat _hitactor) (`GameplayStatics.BreakHitResult` _array_element))
    (if (and (`KismetSystemLibrary.DoesImplementInterface` _hitactor "/Script/arpg_0908.CombatInterface") (`ArpgAbilitySystemLibrary.IsNotFriendBasedOnTag` _hitactor (`self.AvatarCharacter`)))
      (`self.ApplyDamageSingleTarget` _hitactor))))

(fn `ApplyDamageSingleTarget`
  (params (Actor :type "Actor Object Reference"))
  (bind _returnvalue (`self.GetAbilitySystemComponentFromActorInfo`))
  (bind _returnvalue_2 (`AbilitySystemBlueprintLibrary.AssignTagSetByCallerMagnitude` (`AbilitySystemComponent.MakeOutgoingSpec` _returnvalue (`self.DamageEffectClass`) 1.0 (`AbilitySystemComponent.MakeEffectContext` _returnvalue)) (struct :`TagName` "Damage") (`self.GetDamageAtLevel`)))
  (`AbilitySystemComponent.BP_ApplyGameplayEffectSpecToSelf` (`AbilitySystemBlueprintLibrary.GetAbilitySystemComponent` Actor) _returnvalue_2))