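; Gameplay ability that summons a Healing Pylon at the location under the player's mouse.
; After committing, it gets cursor target data, plays the Hook cast montage and waits for that montage's gameplay event.
; On the event, only the authority spawns BP_HealingPylon there, then spawns its default AI controller and starts its blackboard.
; The ability ends when the montage completes.
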(event `self.K2_ActivateAbility`
  (`self.K2_CommitAbility`)
  (bind (_asynctaskproxy _datahandle) (`TargetDataUnderMouse.CreateTargetDataUnderMouse`)
    (:`then`
      (set `self.SummonLocation` (`.Location` (`GameplayStatics.BreakHitResult` (`AbilitySystemBlueprintLibrary.GetHitResultFromTargetData` _datahandle))))
      (`AbilityTask_PlayMontageAndWait.CreatePlayMontageAndWaitProxy` "None" "/Game/Assets/Rawb/Anims/AM_Cast_Hook.AM_Cast_Hook"
        (:`then`
          (`AbilityTask_WaitGameplayEvent.WaitGameplayEvent` (struct :`TagName` "Event.Montage.Hook") null
            (:`then`
              (`self.K2_HasAuthority`
                (:`True`
                  (bind _returnvalue (`ArpgAbilitySystemLibrary.SpawnAIControlledActorAndStartBlackboard` (`self.GetAvatarActorFromActorInfo`) "/Game/Blueprints/Actor/Spawnables/BP_HealingPylon.BP_HealingPylon_C" (`KismetMathLibrary.MakeTransform` (`self.SummonLocation`))))
                  (`Pawn.SpawnDefaultController` _returnvalue)
                  (`arpgAIControlledCharacter.StartBlackboard` _returnvalue))))))
        (:`OnCompleted`
          (`self.K2_EndAbility`))))))