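; Gameplay ability that makes the playable arpgCharacter perform a random dance emote.
; On activation it picks from the avatar's DanceMontages using a random stream seeded by the activation prediction key, so predicting client and server choose alike.
; The random range's inclusive maximum is the array length, so it can land one past the last entry.
; The ability ends when the montage completes, is interrupted or is cancelled.
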(event `self.K2_ActivateAbility`
  (bind _asarpg_character (cast `arpgCharacter` (`self.GetAvatarActorFromActorInfo`))
    (:`then`
      ; Sometimes this interrupts, not sure hwy
      (`AbilityTask_PlayMontageAndWait.CreatePlayMontageAndWaitProxy` "None" (`|GetArrayItem` (`arpgCharacter.DanceMontages` _asarpg_character) (`KismetMathLibrary.RandomIntegerInRangeFromStream` (`KismetMathLibrary.MakeRandomStream` (`ArpgAbilitySystemLibrary.GetAbilityPredictionKey` (`self.CurrentActivationInfo`))) 0 (`KismetArrayLibrary.Array_Length` (`arpgCharacter.DanceMontages` _asarpg_character))))
        (:`OnCompleted`
          _)
        (:`OnInterrupted`
          _)
        (:`OnCancelled`
          _))
      (`self.K2_EndAbility`))
    (:`CastFailed`
      (`KismetSystemLibrary.PrintString` "never should happemn"))))