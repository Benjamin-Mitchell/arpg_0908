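; Channeled Electrocute gameplay ability that shocks the enemy under the mouse with a beam for as long as input is held.
; Mouse target data sets the target and facing, then a montage event disables movement, adds the looping beam cue and starts a repeating damage timer.
; Each tick applies a set-by-caller damage effect to a valid enemy.
; Input release or target death clears the timer, restores movement and cursor, and ends the ability.
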(event `self.K2_ActivateAbility`
  (`self.K2_CommitAbility`)
  (`self.EnforceImplementsCombatInterface`)
  ;[1 1 1 0.5] Store Mouse Data Variables
  (bind (_asynctaskproxy _datahandle) (`TargetDataUnderMouse.CreateTargetDataUnderMouse`)
    (:`ValidData`
      (`self.StoreMouseDataInfo` (`AbilitySystemBlueprintLibrary.GetHitResultFromTargetData` _datahandle))
      (`self.StoreOwnerVariables`)
      (`self.SetEnemyActorIfValid`)
      (`|ExecutionSequence`
        (:`then_0`
          (set `PlayerController.bShowMouseCursor` false (`self.OwnerPlayerController`))
          (message `CombatInterface.UpdateFacingTarget` (`self.GetAvatarActorFromActorInfo`) (`self.MouseHitLocation`))
          (`self.K2_ExecuteGameplayCue` (struct :`TagName` "GameplayCue.ShockBurst"))
          (`AbilityTask_PlayMontageAndWait.CreatePlayMontageAndWaitProxy` "None" (`self.ElectrocuteMontage`) 1.0 "None" false
            (:`then`
              (message `CombatInterface.SetInChannelingLoop` (`self.GetAvatarActorFromActorInfo`) true)
              (`AbilityTask_WaitGameplayEvent.WaitGameplayEvent` (struct :`TagName` "Event.Montage.Electrocute") null
                (:`EventReceived`
                  (`self.SpawnBeam`)
                  (bind _returnvalue (`KismetSystemLibrary.K2_SetTimerDelegate` (delegate `DamageAndCost`) (`self.DamageDeltaTime`) true))
                  (set `self.DamageAndCostTImer` _returnvalue))))))
        (:`then_1`
          (`AbilityTask_WaitInputRelease.WaitInputRelease` false
            (:`OnRelease`
              (`self.ClearTimerAndEndAbility`))))))))

(event `DamageAndCost`
  ;[0.15 0.15 0.15 0.5 10] No Cost currently. Add Cost at the start of this event.
  (if (`KismetSystemLibrary.IsValid` (`self.EnemyActor`))
    (if (`self.TargetDead`)
      (`self.ClearTimerAndEndAbility`)
      (else
        (`self.ApplyDamageSingleTarget` (`self.EnemyActor`))))))

(event `self.PrimaryTargetDied`
  (params (DeadActor :type "Actor Object Reference"))
  ;[0.15 0.15 0.15 0.5 12] TODO: Reroute beam instead of ending ability?
  (`self.ClearTimerAndEndAbility`)
  ;[0.15 0.15 0.15 0.5 12] not currently used because we end ability
  (set `self.TargetDead` false))

(fn `ApplyDamageSingleTarget`
  (params (Actor :type "Actor Object Reference"))
  (locals (TargetActor :type "Actor Object Reference"))
  (bind _returnvalue (`self.GetAbilitySystemComponentFromActorInfo`))
  (set `local.TargetActor` Actor)
  (bind _returnvalue_2 (`AbilitySystemBlueprintLibrary.AssignTagSetByCallerMagnitude` (`AbilitySystemComponent.MakeOutgoingSpec` _returnvalue (`self.DamageEffectClass`) 1.0 (`AbilitySystemComponent.MakeEffectContext` _returnvalue)) (struct :`TagName` "Damage") (`self.GetDamageAtLevel`)))
  (`AbilitySystemComponent.BP_ApplyGameplayEffectSpecToSelf` (`AbilitySystemBlueprintLibrary.GetAbilitySystemComponent` (`local.TargetActor`)) _returnvalue_2))

(fn `ClearTimerAndEndAbility`
  (`KismetSystemLibrary.K2_ClearAndInvalidateTimerHandle` (`self.DamageAndCostTImer`))
  (`self.PrepareToEndAbility`)
  (`self.K2_CommitAbility`)
  (`self.K2_EndAbility`))

(fn `EnforceImplementsCombatInterface`
  (if (not (`KismetSystemLibrary.DoesImplementInterface` (`self.GetAvatarActorFromActorInfo`) "/Script/arpg_0908.CombatInterface"))
    (`self.K2_EndAbility`)))

(fn `PrepareToEndAbility`
  (set `PlayerController.bShowMouseCursor` true (`self.OwnerPlayerController`))
  (message `CombatInterface.SetInChannelingLoop` (`self.GetAvatarActorFromActorInfo`) false)
  (`CharacterMovementComponent.SetMovementMode` (`Character.CharacterMovement` (`self.OwnerCharacter`)) "MOVE_Walking" 0)
  (`self.K2_RemoveGameplayCue` (struct :`TagName` "GameplayCue.ShockLoop")))

(fn `SetEnemyActorIfValid`
  (bind _mousehitactor (`self.MouseHitActor`))
  (if (and (`ArpgAbilitySystemLibrary.IsNotFriendBasedOnTag` (`self.OwnerCharacter`) _mousehitactor) (`KismetSystemLibrary.DoesImplementInterface` _mousehitactor "/Script/arpg_0908.CombatInterface"))
    (set `self.EnemyActor` (`self.MouseHitActor`))))

(fn `SpawnBeam`
  (`CharacterMovementComponent.DisableMovement` (`Character.CharacterMovement` (`self.OwnerCharacter`)))
  (bind _returnvalue (message `CombatInterface.GetWeapon` (`self.GetAvatarActorFromActorInfo`)))
  (`GameplayCueFunctionLibrary.AddGameplayCueOnActor` (`self.GetAvatarActorFromActorInfo`) (struct :`TagName` "GameplayCue.ShockLoop") (`AbilitySystemBlueprintLibrary.MakeGameplayCueParameters` 0.0 0.0 (struct) (struct) (struct) (struct) (struct) (`self.MouseHitLocation`) (0.0 0.0 0.0) null null (`self.EnemyActor`) null 1 1 _returnvalue)))