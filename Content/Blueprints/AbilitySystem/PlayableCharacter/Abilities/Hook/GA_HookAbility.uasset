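; GA_HookAbility is a gameplay ability that fires the playable character's hook projectile toward the location under the mouse.
; It commits, takes target data under the mouse, turns the avatar toward that point through CombatInterface and plays the hook cast montage.
; A montage gameplay event times the projectile spawn from the right-hand socket, avoiding the caster, and the ability ends after a short delay.
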(event `self.K2_ActivateAbility`
  (`self.K2_CommitAbility`)
  (bind (_asynctaskproxy _datahandle) (`TargetDataUnderMouse.CreateTargetDataUnderMouse`)
    (:`ValidData`
      (set `self.ProjectileTargetLocation` (`.Location` (`GameplayStatics.BreakHitResult` (`AbilitySystemBlueprintLibrary.GetHitResultFromTargetData` _datahandle))))
      (bind _ascombat_interface (cast `CombatInterface` (`self.GetAvatarActorFromActorInfo`)))
      (`CombatInterface.UpdateFacingTarget` _ascombat_interface (`self.ProjectileTargetLocation`))
      (`AbilityTask_PlayMontageAndWait.CreatePlayMontageAndWaitProxy` "None" "/Game/Assets/UdemyAssets/Characters/Aura/Animations/Abilities/AM_Cast_Hook.AM_Cast_Hook"
        (:`then`
          (`AbilityTask_WaitGameplayEvent.WaitGameplayEvent` (struct :`TagName` "Event.Montage.Hook") null
            (:`EventReceived`
              (`self.SpawnProjectile` (`self.ProjectileTargetLocation`) (`self.HookWithTags`) (struct) (`|MakeArray` (`self.GetAvatarActorFromActorInfo`)) false (struct :`TagName` "Montage.Attack.RightHand"))
              (`KismetSystemLibrary.Delay` 1.0)
              (`self.K2_EndAbility`))))))))