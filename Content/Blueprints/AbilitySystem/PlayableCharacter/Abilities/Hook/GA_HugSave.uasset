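; Gameplay ability that "hug saves" the character under the mouse by pulling it to the caster.
; It commits, gets cursor target data, turns the avatar to face it and ends if no arpgCharacter was hit.
; DoTheSave sets the target traversing to the caster's location, activates its hook-pull ability by tag, and fires bubble and beam GameplayCues.
; Cast montage and nearest-player radius search are unwired.
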(event `self.K2_ActivateAbility`
  (`self.K2_CommitAbility`)
  (bind (_asynctaskproxy _datahandle) (`TargetDataUnderMouse.CreateTargetDataUnderMouse`)
    (:`ValidData`
      (bind (_bblockinghit _binitialoverlap _time _distance _location _impactpoint _normal _impactnormal _physmat _hitactor) (`GameplayStatics.BreakHitResult` (`AbilitySystemBlueprintLibrary.GetHitResultFromTargetData` _datahandle)))
      (set `self.TargetLocation` _location)
      (bind _ascombat_interface (cast `CombatInterface` (`self.GetAvatarActorFromActorInfo`)))
      (`CombatInterface.UpdateFacingTarget` _ascombat_interface (`self.TargetLocation`))
      (bind _asarpg_character (cast `arpgCharacter` _hitactor)
        (:`then`
          (bind _output_get (set `self.HitActor` _asarpg_character))
          (`self.DoTheSave` _output_get))
        (:`CastFailed`
          ;[0.15 0.15 0.15 0.5 14] TODO: sphere radius, find nearest?
          (`self.K2_EndAbility`))))))

(fn `DoTheSave`
  (params (Target :type "arpgCharacterBase Object Reference"))
  ; Activate Hook-logic
  (`arpgCharacterBase.SetIsTraversing` Target true (`KismetMathLibrary.MakeTransform` (`Actor.K2_GetActorLocation` (`self.GetAvatarActorFromActorInfo`))))
  (`AbilitySystemComponent.TryActivateAbilitiesByTag` (`AbilitySystemBlueprintLibrary.GetAbilitySystemComponent` Target) (`self.HookPullGameplayTag`) true)
  ; Trigger Bubbles
  (`self.K2_ExecuteGameplayCue` (struct :`TagName` "GameplayCue.HugBubble"))
  (`GameplayCueFunctionLibrary.ExecuteGameplayCueOnActor` (`self.HitActor`) (struct :`TagName` "GameplayCue.HugBubble") (`AbilitySystemBlueprintLibrary.MakeGameplayCueParameters` 0.0))
  (`self.K2_ExecuteGameplayCueWithParams` (struct :`TagName` "GameplayCue.HugBeam") (`AbilitySystemBlueprintLibrary.MakeGameplayCueParameters` 0.0 0.0 (struct) (struct) (struct) (struct) (struct) (`Actor.K2_GetActorLocation` (`self.HitActor`))))
  (`self.K2_EndAbility`))