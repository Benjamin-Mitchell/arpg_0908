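; Gameplay ability that plays a playable character's spawn animation, then puts it in play with a random speech line.
; Applies a movement-disabling effect, makes the character visible and plays the montage; completion lifts the block and adds a speech-text gameplay cue.
; The cue's GameplayEffectLevel carries the random line index, and an authority-only timer removes the cue and ends the ability.
; Interruption or cancellation ends the ability without removing the movement block.
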(event `self.K2_ActivateAbility`
  (bind _returnvalue (`self.GetAbilitySystemComponentFromActorInfo`))
  (bind _character (`self.Character`))
  (bind _returnvalue_2 (`AbilitySystemComponent.BP_ApplyGameplayEffectSpecToSelf` _returnvalue (`AbilitySystemComponent.MakeOutgoingSpec` _returnvalue "/Game/Blueprints/AbilitySystem/GeneralEffects/GE_DisableMovement.GE_DisableMovement_C" 0.0 (`AbilitySystemComponent.MakeEffectContext` _returnvalue))))
  (set `self.MovementBlockEffect` _returnvalue_2)
  (bind _asbp_playable_character (cast `/Game/Blueprints/Character/playableCharacter/BP_playableCharacter` (`self.GetAvatarActorFromActorInfo`)))
  (bind _output_get (set `self.Character` _asbp_playable_character))
  (`/Game/Blueprints/Character/playableCharacter/BP_playableCharacter.SetVisible` _output_get)
  (`AbilityTask_PlayMontageAndWait.CreatePlayMontageAndWaitProxy` "None" "/Game/Assets/Rawb/Anims/AM_Rawb_Spawn_01.AM_Rawb_Spawn_01"
    (:`OnCompleted`
      (`self.BP_RemoveGameplayEffectFromOwnerWithHandle` (`self.MovementBlockEffect`))
      (`arpgCharacterBase.SetInPlay` _character true)
      (`self.AddText` _character)
      (`self.K2_HasAuthority`
        (:`True`
          (bind _returnvalue_3 (`KismetSystemLibrary.K2_SetTimerDelegate` (delegate `OnDurationComplete`) (`self.TextVisibilityDuration`)))
          (set `self.Timer` _returnvalue_3))))
    (:`OnInterrupted`
      (`self.K2_EndAbility` :!label _label))
    (:`OnCancelled`
      (goto _label))))

(event `OnDurationComplete`
  (`KismetSystemLibrary.K2_ClearAndInvalidateTimerHandle` (`self.Timer`))
  (`GameplayCueFunctionLibrary.RemoveGameplayCueOnActor` (`self.GetAvatarActorFromActorInfo`) (struct :`TagName` "GameplayCue.SpeechText") (`self.CueParams`))
  (`self.K2_EndAbility`))

(fn `AddText`
  (params (Character :type "/Game/Blueprints/Character/playableCharacter/BP_playableCharacter Object Reference"))
  (bind _output_get (set `self.CueParams` (`AbilitySystemBlueprintLibrary.MakeGameplayCueParameters` 0.0 0.0 (struct) (struct) (struct :`TagName` "Abilities.PlayerInteraction.Spawn") (struct) (struct) (`self.TextOffset`) (0.0 0.0 0.0) (`self.GetAvatarActorFromActorInfo`) null null null (`KismetMathLibrary.RandomIntegerInRange` 0 (`KismetArrayLibrary.Array_Length` (`SpeechStringDataSet.PlayerSpawnSpeechStrings` (`self.SpeechData`)))))))
  (`GameplayCueFunctionLibrary.AddGameplayCueOnActor` Character (struct :`TagName` "GameplayCue.SpeechText") _output_get))