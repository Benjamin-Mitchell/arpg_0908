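; Gameplay ability that starts a hook pull for the playable character.
; On activation it passes the character's traversal target location to UpdateHookPullTarget, then plays the hook montage at increased rate.
; The ability ends when the montage completes, is interrupted or is cancelled.
; Disconnected nodes for applying a hook-pull gameplay effect and fetching a montage through CombatInterface never run.
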(event `self.K2_ActivateAbility`
  (bind _asbp_playable_character (cast `/Game/Blueprints/Character/playableCharacter/BP_playableCharacter` (`self.GetAvatarActorFromActorInfo`)))
  (`arpgCharacterBase.UpdateHookPullTarget` _asbp_playable_character (.location (`arpgCharacterBase.GetTraversalTargetTransform` _asbp_playable_character)))
  (`AbilityTask_PlayMontageAndWait.CreatePlayMontageAndWaitProxy` "None" "/Game/Assets/UdemyAssets/Characters/Aura/Animations/AM_HookAnim.AM_HookAnim" 2.0
    (:`OnCompleted`
      _)
    (:`OnInterrupted`
      _)
    (:`OnCancelled`
      _))
  (`self.K2_EndAbility`))