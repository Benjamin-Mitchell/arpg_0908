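; Cry projectile for the BebeMebe enemy's ability, which deals area damage and leaves a tear area behind.
; All custom logic runs in OnDestroy: it passes each live player within EffectRadius of ArcTargetLocation to DamageTargetASC.
; It then spawns BP_BM_TearArea at the projectile's own transform, passing on its owner as Owner and Instigator, provided that owner is a Pawn.
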(event `self.ReceiveBeginPlay`)

(event `self.OnDestroy`
  (params (OtherActor :type "Actor Object Reference"))
  (bind _returnvalue (`self.GetOwner`))
  (`|ExecutionSequence`
    (:`then_0`
      (bind _outoverlappingactors (`ArpgAbilitySystemLibrary.GetLivePlayersWithinCircleRadius` :`WorldContextObject` self :`Radius` (`self.EffectRadius`) :`SphereOrigin` (`self.ArcTargetLocation`)))
      (for _array_element _outoverlappingactors
        (`self.DamageTargetASC` _array_element)))
    (:`then_1`
      (bind _aspawn (cast `Pawn` _returnvalue))
      (`|SpawnActorFromClass` "/Game/Blueprints/AbilitySystem/Enemy/AbilityActors/BebeMebe/BP_BM_TearArea.BP_BM_TearArea_C" (`self.GetTransform`) "AlwaysSpawn" "MultiplyWithRoot" _returnvalue _aspawn))))

(fn `UserConstructionScript`)