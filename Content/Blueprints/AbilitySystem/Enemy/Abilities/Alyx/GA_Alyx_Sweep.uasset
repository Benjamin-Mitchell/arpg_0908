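; Gameplay ability for the enemy Alyx's spear sweep attack: it faces the combat target and plays the sweep montage.
; The montage's DamageTraceBegin event starts a DetectCollisionBetweenTrace task on the owner's skeletal mesh with intermediate traces, and DamageTraceEnd stops it.
; Actors the trace finds take damage unless tagged as friendly, and the ability ends when the montage completes, is interrupted or is cancelled.
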(event `self.K2_ActivateAbility`
  (bind _returnvalue (`self.GetAvatarActorFromActorInfo`))
  (bind _returnvalue_2 (message `EnemyInterface.GetCombatTarget` _returnvalue))
  (bind _ascombat_interface (cast `CombatInterface` _returnvalue))
  (set `self.TargetLocation` (`Actor.K2_GetActorLocation` _returnvalue_2))
  (`CombatInterface.UpdateFacingTarget` _ascombat_interface (`self.TargetLocation`))
  (`AbilityTask_PlayMontageAndWait.CreatePlayMontageAndWaitProxy` "None" "/Game/Characters/Alyx/Alyx_Anims/AM_Alyx_Spear_Sweep.AM_Alyx_Spear_Sweep"
    (:`then`
      (`AbilityTask_WaitGameplayEvent.WaitGameplayEvent` (struct :`TagName` "Montage.Attack.DamageTraceBegin") null
        (:`then`
          (`AbilityTask_WaitGameplayEvent.WaitGameplayEvent` (struct :`TagName` "Montage.Attack.DamageTraceEnd") null
            (:`EventReceived`
              (`GameplayTask.EndTask` (stale _asynctaskproxy)))))
        (:`EventReceived`
          (bind (_asynctaskproxy _datahandle) (`DetectCollisionBetweenTrace.CreateDetectCollisionBetweenTrace` (`self.GetOwningComponentFromActorInfo`) 3)
            (:`OnCollisionFound`
              (for _array_element (`AbilitySystemBlueprintLibrary.GetActorsFromTargetData` _datahandle)
                (if (`ArpgAbilitySystemLibrary.IsNotFriendBasedOnTag` (`self.GetAvatarActorFromActorInfo`) _array_element)
                  (`self.CauseDamage` _array_element))))))))
    (:`OnCompleted`
      (`self.K2_EndAbility` :!label _label))
    (:`OnInterrupted`
      (goto _label))
    (:`OnCancelled`
      (goto _label))))