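; Gameplay ability for the BebeMebe enemy's kick attack.
; On activation it plays the kick stun montage and waits for the right-foot montage event.
; It then sphere-checks live players around the right-foot combat socket and applies the class-default damage effect to each non-friendly one.
; The ability ends when the montage completes, is interrupted or is cancelled.
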(event `self.K2_ActivateAbility`
  (bind _returnvalue (`self.GetAvatarActorFromActorInfo`))
  (`AbilityTask_PlayMontageAndWait.CreatePlayMontageAndWaitProxy` "None" "/Game/Assets/Suit/Anims/BM_M_Kick_Stun.BM_M_Kick_Stun"
    (:`then`
      (`AbilityTask_WaitGameplayEvent.WaitGameplayEvent` (struct :`TagName` "Montage.Attack.RightFoot") null
        (:`EventReceived`
          (bind _returnvalue_2 (message `CombatInterface.GetCombatSocketLocation` _returnvalue (struct :`TagName` "Montage.Attack.RightFoot")))
          (bind _outoverlappingactors (`ArpgAbilitySystemLibrary.GetLivePlayersWithinSphereRadius` _returnvalue (`|MakeArray` _returnvalue) 50.0 _returnvalue_2))
          (for _array_element _outoverlappingactors
            (if (`ArpgAbilitySystemLibrary.IsNotFriendBasedOnTag` (`self.GetAvatarActorFromActorInfo`) _array_element)
              (`ArpgAbilitySystemLibrary.ApplyDamageEffect` (`self.MakeDamageEffectParamsFromClassDefaults` _array_element)))))))
    (:`OnCompleted`
      (`self.K2_EndAbility` :!label _label))
    (:`OnInterrupted`
      (goto _label))
    (:`OnCancelled`
      (goto _label))))