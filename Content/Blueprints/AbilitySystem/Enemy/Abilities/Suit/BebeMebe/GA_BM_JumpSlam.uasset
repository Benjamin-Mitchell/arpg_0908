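; Gameplay ability for the BM enemy's jump slam, an area attack aimed at its combat target.
; On activation it stores the target's location and feeds it to facing and traverse targets through CombatInterface, falling back to its own location without facing.
; It plays the jump montage and, on the right-hand attack event, damages live players around that stored location rather than the landing position.
; The ability ends when the montage completes, is interrupted or is cancelled.
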(event `self.K2_ActivateAbility`
  (bind _returnvalue (message `EnemyInterface.GetCombatTarget` (`self.GetAvatarActorFromActorInfo`)))
  (`self.SetTargetsIfTargetExists` _returnvalue)
  (`AbilityTask_PlayMontageAndWait.CreatePlayMontageAndWaitProxy` "None" "/Game/Assets/Suit/Anims/AM_BM_Jump_01.AM_BM_Jump_01"
    (:`then`
      (`AbilityTask_WaitGameplayEvent.WaitGameplayEvent` (struct :`TagName` "Montage.Attack.RightHand") null
        (:`EventReceived`
          (bind _outoverlappingactors (`self.GetLiveTargetsInRadius`))
          (for _array_element _outoverlappingactors
            (`ArpgAbilitySystemLibrary.ApplyDamageEffect` (`self.MakeDamageEffectParamsFromClassDefaults` _array_element))))))
    (:`OnCompleted`
      (`self.K2_EndAbility` :!label _label))
    (:`OnInterrupted`
      (goto _label))
    (:`OnCancelled`
      (goto _label))))

(fn `GetLiveTargetsInRadius`
  (returns (OutOverlappingActors :type "Array of Actor Object Reference"))
  (bind _returnvalue (`self.GetAvatarActorFromActorInfo`))
  (bind _outoverlappingactors (`ArpgAbilitySystemLibrary.GetLivePlayersWithinCircleRadius` _returnvalue (`|MakeArray` _returnvalue) (`self.DamageRadius`) (`self.TargetLocation`) (`|MakeArray` (`self.EnemyIgnoreTag`)) (`self.ShowDebugSphereForCollision`)))
  (return _outoverlappingactors))

(fn `SetTargetsIfTargetExists`
  (params (Target :type "Actor Object Reference"))
  (bind _targetlocation (`self.TargetLocation`))
  (if (`KismetSystemLibrary.IsValid` Target)
    (set `self.TargetLocation` (`Actor.K2_GetActorLocation` Target))
    (bind _ascombat_interface (cast `CombatInterface` (`self.GetAvatarActorFromActorInfo`)))
    (`CombatInterface.UpdateFacingTarget` _ascombat_interface _targetlocation)
    (`CombatInterface.UpdateTraverseTarget` _ascombat_interface _targetlocation)
    (else
      (set `self.TargetLocation` (`Actor.K2_GetActorLocation` (`self.GetAvatarActorFromActorInfo`)))
      (bind _ascombat_interface_2 (cast `CombatInterface` (`self.GetAvatarActorFromActorInfo`)))
      (`CombatInterface.UpdateTraverseTarget` _ascombat_interface_2 (`self.TargetLocation`)))))