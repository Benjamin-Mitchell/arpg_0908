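; Melee punch gameplay ability for the BebeMebe Suit enemy.
; On activation it turns the avatar toward its combat target and plays a fixed punch montage, ending when the montage completes, is interrupted or is cancelled.
; A right-hand montage gameplay event triggers a small sphere query at that combat socket, applying the class-default damage effect to non-friendly live players.
; Leftover random-montage and CauseDamage nodes never run.
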(event `self.K2_ActivateAbility`
  (bind _returnvalue (`self.GetAvatarActorFromActorInfo`))
  (bind _returnvalue_2 (`self.GetAvatarActorFromActorInfo`))
  (bind _returnvalue_3 (message `EnemyInterface.GetCombatTarget` _returnvalue))
  (bind _ascombat_interface (cast `CombatInterface` _returnvalue))
  (set `self.TargetLocation` (`Actor.K2_GetActorLocation` _returnvalue_3))
  (`CombatInterface.UpdateFacingTarget` _ascombat_interface (`self.TargetLocation`))
  (`AbilityTask_PlayMontageAndWait.CreatePlayMontageAndWaitProxy` "None" "/Game/Assets/Suit/Anims/AM_BM_M_Punch_01_Montage.AM_BM_M_Punch_01_Montage"
    (:`then`
      (`AbilityTask_WaitGameplayEvent.WaitGameplayEvent` (struct :`TagName` "Montage.Attack.RightHand") null
        (:`EventReceived`
          (bind _returnvalue_4 (message `CombatInterface.GetCombatSocketLocation` _returnvalue_2 (struct :`TagName` "Montage.Attack.RightHand")))
          (bind _outoverlappingactors (`ArpgAbilitySystemLibrary.GetLivePlayersWithinRadius` _returnvalue_2 (`|MakeArray` _returnvalue_2) 50.0 _returnvalue_4))
          (for _array_element _outoverlappingactors
            (if (`ArpgAbilitySystemLibrary.IsNotFriendBasedOnTag` (`self.GetAvatarActorFromActorInfo`) _array_element)
              (`ArpgAbilitySystemLibrary.ApplyDamageEffect` (`self.MakeDamageEffectParamsFromClassDefaults` _array_element)))))))
    (:`OnCompleted`
      (`self.K2_EndAbility` :!label _label))
    (:`OnInterrupted`
      (goto _label))
    (:`OnCancelled`
      (goto _label))))