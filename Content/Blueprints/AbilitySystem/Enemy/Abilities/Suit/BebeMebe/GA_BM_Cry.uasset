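; Enemy gameplay ability for BebeMebe's cry attack, which launches a timed barrage of arcing projectiles.
; It plays the cry montage, waits for the fall-complete montage event, then fires from the right-hand socket tag using RepeatAction.
; Targets cycle between a random navigable point and each player's position, falling back to random when that player is outside Radius.
; Debug spheres and prints trace each shot, and the ability ends after the last.
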(event `self.K2_ActivateAbility`
  (bind _returnvalue (`Actor.K2_GetActorLocation` (`self.GetAvatarActorFromActorInfo`)))
  (`AbilityTask_PlayMontageAndWait.CreatePlayMontageAndWaitProxy` "None" "/Game/Assets/Suit/Anims/AM_BM_Cry01.AM_BM_Cry01"
    (:`then`
      (`AbilityTask_WaitGameplayEvent.WaitGameplayEvent` (struct :`TagName` "Event.Montage.Enemy.BM.CryFallComplete") null
        (:`EventReceived`
          (bind (_asynctaskproxy _actionnumber) (`AbilityTask_Repeat.RepeatAction` (`self.TimestepBetweenProjectiles`) (`self.TotalProjectiles`))
            (:`OnPerformAction`
              (`KismetSystemLibrary.PrintString` (`KismetStringLibrary.BuildString_Int` "" "repeat: " _actionnumber))
              (bind _returnvalue_2 (mod _actionnumber (+ (`GameplayStatics.GetNumPlayerControllers`) 1)))
              (if (== _returnvalue_2 0)
                (bind _randomlocation (`NavigationSystemV1.K2_GetRandomLocationInNavigableRadius` _returnvalue (`self.Radius`) null null :!label _label))
                (bind _output_get (set `self.TargetLocation` _randomlocation))
                (`KismetSystemLibrary.DrawDebugSphere` _output_get 100.0 12 (struct :`R` 1.0 :`G` 1.0 :`B` 1.0 :`A` 1.0) 0.25)
                (else
                  (bind _output_get_2 (set `self.TargetLocation` (`Actor.K2_GetActorLocation` (`Controller.K2_GetPawn` (`GameplayStatics.GetPlayerController` (- _returnvalue_2 1))))))
                  (if (< (`KismetMathLibrary.VSize` (- _returnvalue _output_get_2)) (`self.Radius`))
                    (`KismetSystemLibrary.DrawDebugSphere` _output_get_2 100.0 12 (struct :`R` 1.0 :`G` 1.0 :`B` 1.0 :`A` 1.0) 0.25)
                    (else
                      (goto _label)))))
              (`self.FireArcingProjectile` (struct :`TagName` "Montage.Attack.RightHand") (`self.TargetLocation`)))
            (:`OnFinished`
              (`KismetSystemLibrary.PrintString` "Complete")
              (`self.K2_EndAbility`))))))))