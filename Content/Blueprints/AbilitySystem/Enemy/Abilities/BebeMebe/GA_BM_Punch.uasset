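; GA_BM_Punch is the BebeMebe enemy's melee punch gameplay ability.
; On activation it turns the avatar toward its combat target through CombatInterface and plays the punch montage, ending when the montage completes, is interrupted or is cancelled.
; A right-hand montage gameplay event triggers a small sphere query at the combat socket, applying the class-default damage effect to live non-friendly actors found there.
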(event `self.K2_ActivateAbility`
  (bind _returnvalue (`self.GetAvatarActorFromActorInfo`))
  (bind _returnvalue_2 (message `EnemyInterface.GetCombatTarget` (`self.GetAvatarActorFromActorInfo`)))
  (`self.RotateToTargetIfExists` _returnvalue_2 _returnvalue_2)
  (`AbilityTask_PlayMontageAndWait.CreatePlayMontageAndWaitProxy` "None" "/Game/Assets/Suit/Anims/AM_BM_M_Punch_01_Montage.AM_BM_M_Punch_01_Montage"
    (:`then`
      (`AbilityTask_WaitGameplayEvent.WaitGameplayEvent` (struct :`TagName` "Montage.Attack.RightHand") null
        (:`EventReceived`
          (bind _returnvalue_3 (message `CombatInterface.GetCombatSocketLocation` _returnvalue (struct :`TagName` "Montage.Attack.RightHand")))
          (bind _outoverlappingactors (`ArpgAbilitySystemLibrary.GetLivePlayersWithinSphereRadius` _returnvalue (`|MakeArray` _returnvalue) 50.0 _returnvalue_3))
          (for _array_element _outoverlappingactors
            (if (`ArpgAbilitySystemLibrary.IsNotFriendBasedOnTag` (`self.GetAvatarActorFromActorInfo`) _array_element)
              (`ArpgAbilitySystemLibrary.ApplyDamageEffect` (`self.MakeDamageEffectParamsFromClassDefaults` _array_element)))))))
    (:`OnCompleted`
      (`self.K2_EndAbility` :!label _label))
    (:`OnInterrupted`
      (goto _label))
    (:`OnCancelled`
      (goto _label))))

(fn `RotateToTargetIfExists`
  (params (Object :type "Object Object Reference") (self2 :type "Actor Object Reference"))
  (if (`KismetSystemLibrary.IsValid` Object)
    (bind _ascombat_interface (cast `CombatInterface` (`self.GetAvatarActorFromActorInfo`)))
    (`CombatInterface.UpdateFacingTarget` _ascombat_interface (`Actor.K2_GetActorLocation` self2))))