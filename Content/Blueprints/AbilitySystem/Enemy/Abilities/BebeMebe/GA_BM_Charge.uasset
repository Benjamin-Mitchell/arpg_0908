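; Gameplay ability for the BabyMaybe enemy that charges its combat target, grabs it and throws it.
; A timer drives AI pursuit at boosted speed while a run montage repeats, until in range or timed out.
; Grab montage events disable the target and timer-snap it to the hand socket, rather than attaching it.
; Spin-throw events apply slam damage and lerp the target to a payload offset for throw damage, both with Burn.
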(event `self.K2_ActivateAbility`
  (bind _charactermovement (`Character.CharacterMovement` (`self.BP_BabyMaybe`)))
  (`self.InitVariables`)
  (`self.RepeatPlayMontage`)
  (bind _asbp_baby_maybe (cast `/Game/Blueprints/Enemies/Suits/BabyMaybe/BP_BabyMaybe` (`self.GetAvatarActorFromActorInfo`))
    (:`then`
      (set `self.BP_BabyMaybe` _asbp_baby_maybe)
      (bind _returnvalue (message `EnemyInterface.GetCombatTarget` (`self.BP_BabyMaybe`)))
      (bind _asarpg_character_base (cast `arpgCharacterBase` _returnvalue)
        (:`then`
          (bind _output_get (set `self.CombatTarget` _asarpg_character_base))
          (message `CombatInterface.UpdateFacingTarget` (`self.GetAvatarActorFromActorInfo`) (`Actor.K2_GetActorLocation` _output_get))
          (set `self.PrevModifyMaxWalkSpeed` (`CharacterMovementComponent.MaxWalkSpeed` _charactermovement))
          (set `CharacterMovementComponent.MaxWalkSpeed` (`self.ChargeSpeed`) _charactermovement)
          (bind _returnvalue_2 (`KismetSystemLibrary.K2_SetTimerDelegate` (delegate `Update`) (`self.UpdateRefreshRate`) true))
          (set `self.UpdateTimer` _returnvalue_2))
        (:`CastFailed`
          (`KismetSystemLibrary.PrintString` "Combat Target Cast Failed in Charge Ability!"))))
    (:`CastFailed`
      (`KismetSystemLibrary.PrintString` "ERROR. GA_BM_Charge Activated by someone that isn't BabyMaybe"))))

(event `Update`
  (`AIController.MoveToLocation` (`AIBlueprintHelperLibrary.GetAIController` (`self.BP_BabyMaybe`)) (`Actor.K2_GetActorLocation` (`self.CombatTarget`)) -1.0 true true false true null true)
  (if (< (`KismetMathLibrary.VSize` (- (`Actor.K2_GetActorLocation` (`self.CombatTarget`)) (`Actor.K2_GetActorLocation` (`self.GetAvatarActorFromActorInfo`)))) (`self.AcceptableRange`))
    (`self.EndChargeLoop`)
    (else
      (bind _output_get (set `self.TotalRunDuration` (+ (`self.TotalRunDuration`) (`self.UpdateRefreshRate`))))
      (if (> _output_get (`self.MaxRunDuration`))
        (`self.EndChargeLoop`)
        (`self.K2_EndAbility`)))))

(event `ExecuteSnapping`
  (`self.SnapTargetPositionAndLocation`))

(event `RepeatPlayMontage`
  (bind _returnvalue (`self.GetAvatarActorFromActorInfo`))
  (bind _returnvalue_2 (`Actor.K2_GetActorLocation` (`self.CombatTarget`)))
  (bind (_returnvalue_x _returnvalue_y) (`KismetMathLibrary.BreakVector` (- (`Actor.K2_GetActorLocation` (`self.BP_BabyMaybe`)) _returnvalue_2)))
  (if (`self.EndMontageLoop`)
    (message `CombatInterface.UpdateTraverseTarget` (`self.BP_BabyMaybe`) (+ (* (`KismetMathLibrary.Normal` (`KismetMathLibrary.MakeVector` _returnvalue_x _returnvalue_y)) 150.0) _returnvalue_2))
    (`AbilityTask_PlayMontageAndWait.CreatePlayMontageAndWaitProxy` "None" "/Game/Assets/Rawb/Anims/BM_M_Grab.BM_M_Grab"
      (:`then`
        (`AbilityTask_WaitGameplayEvent.WaitGameplayEvent` (struct :`TagName` "Montage.Attack.RightHand") null true
          (:`EventReceived`
            (`self.DisableTargetActorMovement`)
            (`arpgCharacterBase.ServerSetClientBeginSnapToTargetSocket` (`self.CombatTarget`) (`self.BP_BabyMaybe`) "RightHandSocket" -1.0)
            (bind _returnvalue_3 (`KismetSystemLibrary.K2_SetTimerDelegate` (delegate `ExecuteSnapping`) (`self.TraversalLoopStep`) true true))
            (set `self.SnapCombatTargetLocationTimerHandle` _returnvalue_3))))
      (:`OnCompleted`
        (bind _returnvalue_4 (`ArpgAbilitySystemLibrary.GetFloorPositionBelowLocation` _returnvalue (`Actor.K2_GetActorLocation` _returnvalue) 1500.0))
        (set `self.MontageActivationActorLocation` _returnvalue_4)
        (`AbilityTask_PlayMontageAndWait.CreatePlayMontageAndWaitProxy` "None" "/Game/Assets/Rawb/Anims/AM_BM_M_SpinThrow1_Montage.AM_BM_M_SpinThrow1_Montage"
          (:`then`
            (bind (_asynctaskproxy _payload) (`AbilityTask_WaitGameplayEvent.WaitGameplayEvent` (struct :`TagName` "Montage.Offset.1") null true)
              (:`then`
                (`AbilityTask_WaitGameplayEvent.WaitGameplayEvent` (struct :`TagName` "Montage.Attack.Head") null
                  (:`EventReceived`
                    (`self.ApplySlamDamage`))))
              (:`EventReceived`
                ; Stop Snapping Combat Target Location
                (`arpgCharacterBase.ServerSetClientEndSnapToTargetSocket` (`self.CombatTarget`))
                (`KismetSystemLibrary.K2_ClearAndInvalidateTimerHandle` (`self.SnapCombatTargetLocationTimerHandle`))
                (set `self.TargetInitialLocation` (`Actor.K2_GetActorLocation` (`self.CombatTarget`)))
                (bind _asbp_location_payload (cast `/Game/Blueprints/AnimNotifies/BP_LocationPayload` (`.OptionalObject` (break `GameplayEventData` _payload))))
                (bind _output_get (set `self.LocationPayload` _asbp_location_payload))
                (set `self.TraversalTarget` (+ (`/Game/Blueprints/AnimNotifies/BP_LocationPayload.LocationOffset` _output_get) (`self.MontageActivationActorLocation`) (`KismetMathLibrary.MakeVector` 0.0 0.0 (`CapsuleComponent.CapsuleHalfHeight` (`Character.CapsuleComponent` (`self.CombatTarget`))))))
                (bind _returnvalue_5 (`KismetSystemLibrary.K2_SetTimerDelegate` (delegate `LerpToTarget`) (`self.TraversalLoopStep`) true true))
                (set `self.TraversalTimerHandle` _returnvalue_5))))
          (:`OnCompleted`
            ; TODO: How to re-enable movement?
            (`AbilitySystemComponent.RemoveActiveEffectsWithGrantedTags` (`AbilitySystemBlueprintLibrary.GetAbilitySystemComponent` (`self.CombatTarget`)) (struct :`GameplayTags` (struct :`(TagName` "Player.Block.InputHeld") :`(TagName` "Player.Block.InputPressed") :`(TagName` "Player.Block.InputReleased") :`(TagName` "Player.Block.Rotation"))))
            (`self.K2_EndAbility`)))))
    (else
      (bind _asynctaskproxy_2 (`AbilityTask_PlayMontageAndWait.CreatePlayMontageAndWaitProxy` "None" "/Game/Assets/Rawb/Anims/AM_BM_M_Grab_Run_01.AM_BM_M_Grab_Run_01")
        (:`then`
          (set `self.PlayMontageTask` _asynctaskproxy_2))
        (:`OnBlendOut`
          (`self.RepeatPlayMontage`))
        (:`OnInterrupted`
          (`KismetSystemLibrary.PrintString` "Interrupted!"))
        (:`OnCancelled`
          (`KismetSystemLibrary.PrintString` "Cancelled!"))))))

(event `LerpToTarget`
  (set `self.TraversalDurationSoFar` (+ (`self.TraversalDurationSoFar`) (`self.TraversalLoopStep`)))
  (`Actor.K2_SetActorLocation` (`self.CombatTarget`) (`|EaseFunction` "Linear" (/ (`self.TraversalDurationSoFar`) (`/Game/Blueprints/AnimNotifies/BP_LocationPayload.TraversalDuration` (`self.LocationPayload`))) (`self.TargetInitialLocation`) (`self.TraversalTarget`)) false false)
  (if (>= (`self.TraversalDurationSoFar`) (`/Game/Blueprints/AnimNotifies/BP_LocationPayload.TraversalDuration` (`self.LocationPayload`)))
    (`self.ApplyThrowDamage`)
    (`KismetSystemLibrary.K2_ClearAndInvalidateTimerHandle` (`self.TraversalTimerHandle`))))

(fn `ApplySlamDamage`
  (bind _returnvalue (`self.GetAvatarActorFromActorInfo`))
  (`ArpgAbilitySystemLibrary.ApplyDamageEffect` (make `DamageEffectParams` _returnvalue "/Game/Blueprints/AbilitySystem/GeneralEffects/GE_Damage.GE_Damage_C" (`AbilitySystemBlueprintLibrary.GetAbilitySystemComponent` _returnvalue) (`AbilitySystemBlueprintLibrary.GetAbilitySystemComponent` (`self.CombatTarget`)) (`.Value` (break `ScalableFloat` (`self.SlamDamage`))) 1.0 (`|MakeArray` (make `DebuffInfo` (struct :`TagName` "Debuff.Burn") 3.0 0.5 100.0 2.0)) 150.0 (0.0 0.0 300.0) 0.0)))

(fn `ApplyThrowDamage`
  (bind _returnvalue (`self.GetAvatarActorFromActorInfo`))
  (`ArpgAbilitySystemLibrary.ApplyDamageEffect` (make `DamageEffectParams` _returnvalue "/Game/Blueprints/AbilitySystem/GeneralEffects/GE_Damage.GE_Damage_C" (`AbilitySystemBlueprintLibrary.GetAbilitySystemComponent` _returnvalue) (`AbilitySystemBlueprintLibrary.GetAbilitySystemComponent` (`self.CombatTarget`)) (`.Value` (break `ScalableFloat` (`self.ThrowDamage`))) 1.0 (`|MakeArray` (make `DebuffInfo` (struct :`TagName` "Debuff.Burn") 3.0 0.5 100.0 2.0)) 150.0 (0.0 0.0 300.0) 0.0)))

(fn `DisableTargetActorMovement`
  (locals (InitialCharacterScale :type "Vector Structure" :default (0.0 0.0 0.0)))
  (bind _returnvalue (`AbilitySystemBlueprintLibrary.GetAbilitySystemComponent` (`self.CombatTarget`)))
  (bind (_returnvalue_x _returnvalue_y) (`KismetMathLibrary.BreakVector` (- (`Actor.K2_GetActorLocation` (`self.GetAvatarActorFromActorInfo`)) (`Actor.K2_GetActorLocation` (`self.CombatTarget`)))))
  ; DisablePlayerInputs
  (`AbilitySystemComponent.BP_ApplyGameplayEffectSpecToSelf` _returnvalue (`AbilitySystemComponent.MakeOutgoingSpec` _returnvalue "/Game/Blueprints/AbilitySystem/GeneralEffects/GE_DisableMovement.GE_DisableMovement_C" 0.0 (`AbilitySystemComponent.MakeEffectContext` (`self.GetAbilitySystemComponentFromActorInfo`))))
  ; DisableMovement
  (`CharacterMovementComponent.SetMovementMode` (`Character.CharacterMovement` (`self.CombatTarget`)) "MOVE_None" 0)
  ; Disable Target Collision
  (`PrimitiveComponent.SetCollisionEnabled` (`Character.CapsuleComponent` (`self.CombatTarget`)) "NoCollision")
  (set `self.SnapCombatTargetLocationTimerHandle` (struct))
  (bind _asbp_arpg_player_controller (cast `/Game/Blueprints/Player/BP_ArpgPlayerController` (`Pawn.GetController` (`self.CombatTarget`))))
  (`/Game/Blueprints/Player/BP_ArpgPlayerController.SetCameraTransitionViaOffset` :`self` _asbp_arpg_player_controller :`TransitionOffset` (`KismetMathLibrary.MakeVector` _returnvalue_x _returnvalue_y) :`InTransitionDuration` 0.5))

(fn `EndChargeLoop`
  (set `CharacterMovementComponent.MaxWalkSpeed` (`self.PrevModifyMaxWalkSpeed`) (`Character.CharacterMovement` (`self.BP_BabyMaybe`)))
  (set `self.EndMontageLoop` true)
  (`KismetSystemLibrary.K2_ClearAndInvalidateTimerHandle` (`self.UpdateTimer`)))

(fn `InitVariables`
  (set `self.EndMontageLoop` false)
  (set `self.TotalRunDuration` 0.0))

(fn `SnapTargetPositionAndLocation`
  (bind _combattarget (`self.CombatTarget`))
  (bind (_returnvalue_location _returnvalue_rotation _returnvalue_scale) (`KismetMathLibrary.BreakTransform` (`Actor.GetTransform` _combattarget)))
  (bind (_returnvalue_location_2 _returnvalue_rotation_2) (`KismetMathLibrary.BreakTransform` (`SceneComponent.GetSocketTransform` (`Character.Mesh` (`self.BP_BabyMaybe`)) "RightHandSocket" "RTS_World")))
  (`Actor.K2_SetActorTransform` _combattarget (`KismetMathLibrary.MakeTransform` _returnvalue_location_2 _returnvalue_rotation_2 _returnvalue_scale) false false))

(fn `StartChargeMontageLoop`)