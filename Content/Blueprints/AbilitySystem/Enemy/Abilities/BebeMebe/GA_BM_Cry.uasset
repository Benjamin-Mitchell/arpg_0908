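; Enemy gameplay ability for BebeMebe's cry attack, which lobs a timed series of arcing projectiles around the caster.
; It plays the cry montage, waits for its fall-complete gameplay event, then fires via a RepeatAction task and ends when finished.
; Shots cycle between a random navigable point and each player's pawn, snapped to the floor below.
; Players outside the radius are replaced by random points.
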(event `self.K2_ActivateAbility`
  (bind _returnvalue (`Actor.K2_GetActorLocation` (`self.GetAvatarActorFromActorInfo`)))
  (`AbilityTask_PlayMontageAndWait.CreatePlayMontageAndWaitProxy` "None" "/Game/Assets/Suit/Anims/AM_BM_Cry01.AM_BM_Cry01"
    (:`then`
      (`AbilityTask_WaitGameplayEvent.WaitGameplayEvent` (struct :`TagName` "Event.Montage.Enemy.BM.CryFallComplete") null
        (:`EventReceived`
          (bind (_asynctaskproxy _actionnumber) (`AbilityTask_Repeat.RepeatAction` (`self.TimestepBetweenProjectiles`) (`self.TotalProjectiles`))
            (:`OnPerformAction`
              (bind _returnvalue_2 (mod _actionnumber (+ (`GameplayStatics.GetNumPlayerControllers`) 1)))
              (if (== _returnvalue_2 0)
                (bind _randomlocation (`NavigationSystemV1.K2_GetRandomLocationInNavigableRadius` _returnvalue (`self.Radius`) null null :!label _label))
                (set `self.TargetLocation` _randomlocation)
                (else
                  (bind _returnvalue_3 (`Controller.K2_GetPawn` (`GameplayStatics.GetPlayerController` (- _returnvalue_2 1))))
                  (set `self.TargetActor` _returnvalue_3)
                  (bind _output_get (set `self.TargetLocation` (`Actor.K2_GetActorLocation` _returnvalue_3)))
                  (if (< (`KismetMathLibrary.VSize` (- _returnvalue _output_get)) (`self.Radius`))
                    (bind _returnvalue_4 (`ArpgAbilitySystemLibrary.GetFloorPositionBelowLocation` (`self.GetAvatarActorFromActorInfo`) (`self.TargetLocation`)))
                    (set `self.TargetLocation` _returnvalue_4)
                    (else
                      (goto _label)))))
              (`self.FireArcingProjectile` (struct :`TagName` "Montage.Attack.RightHand") (`self.TargetLocation`)))
            (:`OnFinished`
              (`self.K2_EndAbility`))))))))