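; BebeMebe enemy gameplay ability that performs a repeated fire breath cast, sweeping the caster around during the montage.
; The first cast targets the current combat target; each repeat targets the previous cast location with an added rotation offset.
; A looping timer applies stepped actor rotation, gated on and off by two montage offset gameplay events.
; Montage completion recursively starts the next cast until the loop count is reached, then ends the ability.
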(event `self.K2_ActivateAbility`
  (bind _returnvalue (`self.GetAvatarActorFromActorInfo`))
  (`KismetSystemLibrary.K2_SetTimerDelegate` (delegate `RotateCaster`) (`self.RotationDeltaTime`) true)
  (set `self.PreviousCastLocation` (`Actor.K2_GetActorLocation` _returnvalue))
  (bind _returnvalue_2 (message `EnemyInterface.GetCombatTarget` _returnvalue))
  (`self.SetTargetsIfTargetExists` false _returnvalue_2 (struct) false true)
  (`self.ExecuteALoop`))

(event `RotateCaster`
  (if (`self.ShouldRotate`)
    (`Actor.K2_AddActorWorldRotation` (`self.GetAvatarActorFromActorInfo`) (`self.PerStepRotation`) false false)))

(event `ExecuteALoop`
  (`AbilityTask_PlayMontageAndWait.CreatePlayMontageAndWaitProxy` "None" "/Game/Assets/Rawb/Anims/AM_BM_M_FireBreath1.AM_BM_M_FireBreath1"
    (:`then`
      (`AbilityTask_WaitGameplayEvent.WaitGameplayEvent` (struct :`TagName` "Montage.Offset.1") null
        (:`then`
          (`AbilityTask_WaitGameplayEvent.WaitGameplayEvent` (struct :`TagName` "Montage.Offset.2") null
            (:`EventReceived`
              (set `self.ShouldRotate` false))))
        (:`EventReceived`
          (set `self.ShouldRotate` true))))
    (:`OnCompleted`
      (if (>= (`self.NumLoopSoFar`) (`self.TotalLoops`))
        (`self.K2_EndAbility`)
        (else
          (`self.SetTargetsBasedOnInputLocation` false (`self.PreviousCastLocation`) (`self.PerCastRotationOffset`) true)
          (set `self.PreviousCastLocation` (`Actor.K2_GetActorLocation` (`self.GetAvatarActorFromActorInfo`)))
          (`/Engine/EditorBlueprintResources/StandardMacros.IncrementInt` (`self.NumLoopSoFar`)
            (:`  `
              (`self.ExecuteALoop`))))))))