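; Enemy gameplay ability for BebeMebe that performs a jump slam dealing area damage around the enemy.
; On activation it sets targets from the avatar's combat target, snapped to the floor, and plays the jump montage.
; A montage gameplay event triggers damage effects, built from class defaults, on live players within the damage radius, excluding tagged actors.
; The ability ends when the montage completes, is interrupted or is cancelled.
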(event `self.K2_ActivateAbility`
  (bind _returnvalue (message `EnemyInterface.GetCombatTarget` (`self.GetAvatarActorFromActorInfo`)))
  (`self.SetTargetsIfTargetExists` true _returnvalue)
  (`AbilityTask_PlayMontageAndWait.CreatePlayMontageAndWaitProxy` "None" "/Game/Assets/Suit/Anims/AM_BM_Jump_01.AM_BM_Jump_01"
    (:`then`
      (`AbilityTask_WaitGameplayEvent.WaitGameplayEvent` (struct :`TagName` "Montage.Attack.RightHand") null
        (:`EventReceived`
          (bind _outoverlappingactors (`self.GetLiveTargetsInRadius`))
          (for _array_element _outoverlappingactors
            (`ArpgAbilitySystemLibrary.ApplyDamageEffect` (`self.MakeDamageEffectParamsFromClassDefaults` _array_element))))))
    (:`OnCompleted`
      (`self.K2_EndAbility` :!label _label))
    (:`OnInterrupted`
      (goto _label))
    (:`OnCancelled`
      (goto _label))))

(fn `GetLiveTargetsInRadius`
  (returns (OutOverlappingActors :type "Array of Actor Object Reference"))
  (bind _returnvalue (`self.GetAvatarActorFromActorInfo`))
  (bind _outoverlappingactors (`ArpgAbilitySystemLibrary.GetLivePlayersWithinCircleRadius` _returnvalue (`|MakeArray` _returnvalue) (`self.DamageRadius`) (`Actor.K2_GetActorLocation` (`self.GetAvatarActorFromActorInfo`)) (`|MakeArray` (`self.EnemyIgnoreTag`)) (`self.ShowDebugSphereForCollision`)))
  (return _outoverlappingactors))