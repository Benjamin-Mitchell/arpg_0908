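; BebeMebe enemy dash attack ability that damages players caught along the dash.
; On activation it sets targets from the combat target with a 180-degree rotation offset, disables pawn capsule collision and plays the cry-dash montage.
; Montage gameplay events start and stop a looping timer that sphere-checks around the upper-chest socket, damaging each non-friendly live player once via HitActorArray.
; Montage completion, interruption or cancellation restores collision and ends the ability.
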(event `self.K2_ActivateAbility`
  (bind _asarpg_character_base (cast `arpgCharacterBase` (`self.GetAvatarActorFromActorInfo`)))
  (bind _output_get (set `self.CasterArpgCharacterBase` _asarpg_character_base))
  (`arpgCharacterBase.SetCapsulePawnCollisionEnabled` _output_get false)
  (bind _returnvalue (message `EnemyInterface.GetCombatTarget` (`self.GetAvatarActorFromActorInfo`)))
  (`self.SetTargetsIfTargetExists` false _returnvalue (struct :`Yaw` 180.0))
  (`AbilityTask_PlayMontageAndWait.CreatePlayMontageAndWaitProxy` "None" "/Game/Assets/Rawb/Anims/AM_BM_B_Cry_Dash1.AM_BM_B_Cry_Dash1"
    (:`then`
      (`AbilityTask_WaitGameplayEvent.WaitGameplayEvent` (struct :`TagName` "Montage.Attack.DamageTraceBegin") null
        (:`then`
          (`AbilityTask_WaitGameplayEvent.WaitGameplayEvent` (struct :`TagName` "Montage.Attack.DamageTraceEnd") null
            (:`EventReceived`
              (`KismetSystemLibrary.K2_ClearAndInvalidateTimerHandle` (`self.CollisionCheckTimer`)))))
        (:`EventReceived`
          (bind _returnvalue_2 (`KismetSystemLibrary.K2_SetTimerDelegate` (delegate `CheckCollision`) (`self.SampleDeltaTime`) true true))
          (set `self.CollisionCheckTimer` _returnvalue_2))))
    (:`OnCompleted`
      (`arpgCharacterBase.SetCapsulePawnCollisionEnabled` (`self.CasterArpgCharacterBase`) true :!label _label)
      (`self.K2_EndAbility`))
    (:`OnInterrupted`
      (goto _label))
    (:`OnCancelled`
      (goto _label))))

(event `CheckCollision`
  (bind _returnvalue (`self.GetAvatarActorFromActorInfo`))
  (bind _returnvalue_2 (message `CombatInterface.GetCombatSocketLocation` _returnvalue (struct :`TagName` "Montage.Attack.UpperChest")))
  (bind _outoverlappingactors (`ArpgAbilitySystemLibrary.GetLivePlayersWithinSphereRadius` _returnvalue (`|MakeArray` _returnvalue) (`self.DamageRadius`) _returnvalue_2))
  (for _array_element _outoverlappingactors
    (set `self.Array Element` _array_element)
    (if (`ArpgAbilitySystemLibrary.IsNotFriendBasedOnTag` (`self.GetAvatarActorFromActorInfo`) _array_element)
      (if (not (`KismetArrayLibrary.Array_Contains` (`self.HitActorArray`) (`self.Array Element`)))
        (`ArpgAbilitySystemLibrary.ApplyDamageEffect` (`self.MakeDamageEffectParamsFromClassDefaults` (`self.Array Element`)))
        (`KismetArrayLibrary.Array_Add` (`self.HitActorArray`) (`self.Array Element`))))))