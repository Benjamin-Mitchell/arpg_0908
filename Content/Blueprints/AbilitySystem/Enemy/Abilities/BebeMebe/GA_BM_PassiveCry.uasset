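; GA_BM_PassiveCry is a gameplay ability for the BebeMebe enemy that fires a series of arcing projectiles around itself.
; On activation, a RepeatAction task fires a set number of shots at a fixed interval.
; Each shot launches from the right-hand montage socket toward a random navigable point within a radius of the avatar.
; Ending the ability also ends the stored repeat task.
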(event `self.K2_ActivateAbility`
  (bind _asynctaskproxy (`AbilityTask_Repeat.RepeatAction` (`self.TimestepBetweenProjectiles`) (`self.TotalProjectiles`))
    (:`then`
      (set `self.RepeatTask` _asynctaskproxy))
    (:`OnPerformAction`
      (bind _randomlocation (`NavigationSystemV1.K2_GetRandomLocationInNavigableRadius` (`Actor.K2_GetActorLocation` (`self.GetAvatarActorFromActorInfo`)) (`self.Radius`) null null))
      (`self.FireArcingProjectile` (struct :`TagName` "Montage.Attack.RightHand") _randomlocation))))

(event `self.K2_OnEndAbility`
  (params (bWasCancelled :type Boolean))
  (`GameplayTask.EndTask` (`self.RepeatTask`)))