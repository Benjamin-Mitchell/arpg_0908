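; Gameplay ability that transforms the BabyMaybe enemy between its two forms, tracked by the IsMaybe flag.
; On activation it clears the NeedsTransform blackboard bool and plays the transform montage matching the current form.
; IsMaybe flips when the montage blends out, or when it is interrupted or cancelled.
; The ability ends on completion, interruption or cancellation.
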(event `self.K2_ActivateAbility`
  (bind _asbp_baby_maybe (cast `/Game/Blueprints/Enemies/BabyMaybe/BP_BabyMaybe` (`self.GetAvatarActorFromActorInfo`)))
  (bind _output_get (set `self.BabyMaybe` _asbp_baby_maybe))
  (`arpgEnemy.SetBlackboardCustomBool` _output_get "NeedsTransform" false)
  (if (`/Game/Blueprints/Enemies/BabyMaybe/BP_BabyMaybe.IsMaybe` (`self.BabyMaybe`))
    (`AbilityTask_PlayMontageAndWait.CreatePlayMontageAndWaitProxy` "None" "/Game/Assets/Rawb/Anims/BM_M_Transform.BM_M_Transform"
      (:`OnCompleted`
        (`self.K2_EndAbility`))
      (:`OnBlendOut`
        (`self.FlipIsMaybe`))
      (:`OnInterrupted`
        (`self.FlipIsMaybe` :!label _label)
        (`self.K2_EndAbility`))
      (:`OnCancelled`
        (goto _label)))
    (else
      (`AbilityTask_PlayMontageAndWait.CreatePlayMontageAndWaitProxy` "None" "/Game/Assets/Rawb/Anims/BM_B_Transform.BM_B_Transform"
        (:`OnCompleted`
          (`self.K2_EndAbility`))
        (:`OnBlendOut`
          (`self.FlipIsMaybe`))
        (:`OnInterrupted`
          (`self.FlipIsMaybe` :!label _label_2)
          (`self.K2_EndAbility`))
        (:`OnCancelled`
          (goto _label_2))))))

(fn `FlipIsMaybe`
  (bind _babymaybe (`self.BabyMaybe`))
  (`/Game/Blueprints/Enemies/BabyMaybe/BP_BabyMaybe.SetIsMaybe` _babymaybe (not (`/Game/Blueprints/Enemies/BabyMaybe/BP_BabyMaybe.IsMaybe` _babymaybe))))