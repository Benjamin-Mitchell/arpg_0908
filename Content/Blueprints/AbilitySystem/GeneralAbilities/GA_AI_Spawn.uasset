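; GA_AI_Spawn is a gameplay ability that runs the spawn sequence for an AI-controlled character.
; It makes the mesh visible and plays the character's spawn montage, if one is set.
; On completion or with no montage, it starts the blackboard and self-applies the spawn effects, calling EndAbility inside that loop.
; An interrupted or cancelled montage prints an error and ends the ability without either step.
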(event `self.K2_ActivateAbility`
  (bind _castingaicharacter (`self.CastingAICharacter`))
  (bind _returnvalue (`KismetSystemLibrary.GetDisplayName` (`self.CastingAICharacter`)))
  (bind _returnvalue_2 (`AbilitySystemBlueprintLibrary.GetAbilitySystemComponent` _castingaicharacter))
  (bind _asarpg_aicontrolled_character (cast `arpgAIControlledCharacter` (`self.GetAvatarActorFromActorInfo`)))
  (bind _output_get (set `self.CastingAICharacter` _asarpg_aicontrolled_character))
  ;[0.15 0.15 0.15 0.5 14] As long as the Mesh is replicated, this will update on clients too.
  (`SceneComponent.SetVisibility` (`Character.Mesh` _output_get) true false)
  (bind _spawnanimation (`arpgAIControlledCharacter.SpawnAnimation` _output_get))
  (if (`KismetSystemLibrary.IsValid` _spawnanimation)
    (`AbilityTask_PlayMontageAndWait.CreatePlayMontageAndWaitProxy` "None" _spawnanimation
      (:`OnCompleted`
        (`arpgAIControlledCharacter.StartBlackboard` (`self.CastingAICharacter`) :!label _label)
        (bind _returnvalue_3 (`arpgAIControlledCharacter.GetSpawnEffects` _castingaicharacter))
        (for _array_element _returnvalue_3
          (`AbilitySystemComponent.BP_ApplyGameplayEffectSpecToSelf` _returnvalue_2 (`AbilitySystemComponent.MakeOutgoingSpec` _returnvalue_2 _array_element 0.0 (`AbilitySystemComponent.MakeEffectContext` (`AbilitySystemBlueprintLibrary.GetAbilitySystemComponent` _castingaicharacter))))
          (`self.K2_EndAbility`)))
      (:`OnInterrupted`
        (`KismetSystemLibrary.PrintString` (`KismetStringLibrary.Concat_StrStr` "ERROR: Spawn Anim was interrupted for character: " _returnvalue) true true (struct :`G` 0.66 :`B` 1.0 :`A` 1.0) 8.0)
        (`self.K2_EndAbility` :!label _label_2))
      (:`OnCancelled`
        (`KismetSystemLibrary.PrintString` (`KismetStringLibrary.Concat_StrStr` "ERROR: Spawn Anim was Cancelled for character: " _returnvalue) true true (struct :`G` 0.66 :`B` 1.0 :`A` 1.0) 8.0)
        (goto _label_2)))
    (else
      (goto _label))))