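; BP_FXTrail is a timed-effect anim notify state that drives a trail VFX between two mesh sockets during an animation.
; Each notify tick, it gets the spawned effect and writes the VFXStart and VFXEnd socket locations into its FXStartTrail and FXEndTrail vector parameters.
; If no valid effect exists, it prints a failure message.
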(fn `Received_NotifyTick`
  (params (MeshComp :type "SkeletalMeshComponent Object Reference") (Animation :type "AnimSequenceBase Object Reference") (FrameDeltaTime :type "Float (single-precision)") (EventReference :type "AnimNotifyEventReference Structure (by ref)"))
  (returns (ReturnValue :type Boolean))
  (bind _returnvalue (`self.GetSpawnedEffect` MeshComp))
  (`/Engine/EditorBlueprintResources/StandardMacros.IsValid` _returnvalue
    (:`Is Valid`
      (`FXSystemComponent.SetVectorParameter` _returnvalue "FXStartTrail" (`SceneComponent.GetSocketLocation` MeshComp (`self.VFX_Start`)))
      (`FXSystemComponent.SetVectorParameter` _returnvalue "FXEndTrail" (`SceneComponent.GetSocketLocation` MeshComp (`self.VFX_End`)))
      (return false))
    (:`Is Not Valid`
      (`KismetSystemLibrary.PrintString` null "Failure")
      (return false))))