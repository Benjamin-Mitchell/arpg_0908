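; BP_Hole is a hole actor in the virtual texture material function folder, built from a Mesh component and an Overlay component.
; Its construction script assigns the HoleMesh variable to both components, then applies the Material variable to Mesh and M_HoleOverlay to Overlay, so both share one shape with different materials.
; It has no active runtime logic, as the event graph holds only disabled placeholder events.
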(fn `UserConstructionScript`
  (`StaticMeshComponent.SetStaticMesh` (`self.Mesh`) (`self.Hole_Mesh`))
  (`PrimitiveComponent.SetMaterial` (`self.Mesh`) 0 (`self.Material`))
  (`StaticMeshComponent.SetStaticMesh` (`self.Overlay`) (`self.Hole_Mesh`))
  (`PrimitiveComponent.SetMaterial` (`self.Overlay`) 0 "/Game/VFX/Material/MaterialFunctions/VirtualTexture/M_HoleOverlay.M_HoleOverlay"))