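; Demo actor in a VFX material-function pack that moves four meshes, apparently to showcase a sprite distortion material effect.
; On BeginPlay, one timeline starts and its Movement track drives a lerp that slides all four meshes between two relative X positions.
; Each mesh keeps its own Y and Z, and every update moves it with teleport enabled.
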(event `self.ReceiveTick`
  (params (DeltaSeconds :type "Float (single-precision)")))

(event `self.ReceiveBeginPlay`
  (bind _movemesh_3 (`self.MoveMesh 3`))
  (bind _movemesh_2 (`self.MoveMesh 2`))
  (bind _movemesh_4 (`self.MoveMesh 4`))
  (bind _movemesh_1 (`self.MoveMesh 1`))
  (bind (_relativelocation_x _relativelocation_y _relativelocation_z) (`KismetMathLibrary.BreakVector` (`SceneComponent.RelativeLocation` _movemesh_4)))
  (bind (_relativelocation_x_2 _relativelocation_y_2 _relativelocation_z_2) (`KismetMathLibrary.BreakVector` (`SceneComponent.RelativeLocation` _movemesh_1)))
  (bind (_relativelocation_x_3 _relativelocation_y_3 _relativelocation_z_3) (`KismetMathLibrary.BreakVector` (`SceneComponent.RelativeLocation` _movemesh_2)))
  (bind (_relativelocation_x_4 _relativelocation_y_4 _relativelocation_z_4) (`KismetMathLibrary.BreakVector` (`SceneComponent.RelativeLocation` _movemesh_3)))
  (bind (_direction _movement) (`Timeline|Timeline_0` :!via `PlayFromStart`)
    (:`Update`
      (bind _returnvalue (`KismetMathLibrary.Lerp` -500.0 500.0 _movement))
      (`SceneComponent.K2_SetRelativeLocation` _movemesh_1 (`KismetMathLibrary.MakeVector` _returnvalue _relativelocation_y_2 _relativelocation_z_2) false true)
      (`SceneComponent.K2_SetRelativeLocation` _movemesh_2 (`KismetMathLibrary.MakeVector` _returnvalue _relativelocation_y_3 _relativelocation_z_3) false true)
      (`SceneComponent.K2_SetRelativeLocation` _movemesh_3 (`KismetMathLibrary.MakeVector` _returnvalue _relativelocation_y_4 _relativelocation_z_4) false true)
      (`SceneComponent.K2_SetRelativeLocation` _movemesh_4 (`KismetMathLibrary.MakeVector` _returnvalue _relativelocation_y _relativelocation_z) false true))))

(fn `UserConstructionScript`)