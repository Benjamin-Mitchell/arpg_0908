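; Chaos field actor that blasts apart fracturable geometry when its Explode event is called.
; Explode plays a demon hurt sound, waits briefly, then applies two physics fields sized and centered on its Sphere component.
; A radial falloff drives external cluster strain to break clusters, then a culled radial vector applies linear velocity to push pieces outward.
; The Niagara spawn and DestroyActor nodes are disconnected and never run.
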(event `Explode`
  (bind _fieldsystemcomponent (`self.FieldSystemComponent`))
  (bind _sphere (`self.Sphere`))
  (bind _returnvalue (`SceneComponent.K2_GetComponentLocation` _sphere))
  (bind _returnvalue_2 (`RadialFalloff.SetRadialFalloff` (`self.RadialFalloff`) 500000.0 0.0 1.0 0.0 (`SphereComponent.GetScaledSphereRadius` _sphere) _returnvalue "Field_FallOff_None"))
  (`GameplayStatics.PlaySoundAtLocation` "/Game/Assets/UdemyAssets/Sounds/Enemies/Demon/Hurt/SFX_Demon_Hurt_01.SFX_Demon_Hurt_01" (`KismetMathLibrary.MakeVector` (.x (`self.K2_GetActorLocation`)) (.y (`self.K2_GetActorLocation`)) (.z (`self.K2_GetActorLocation`))) (struct) 1.0 1.0 0.0 null null null null)
  (`KismetSystemLibrary.Delay` 0.15)
  (`FieldSystemComponent.ApplyPhysicsField` _fieldsystemcomponent true "Field_ExternalClusterStrain" null _returnvalue_2)
  (`FieldSystemComponent.ApplyPhysicsField` _fieldsystemcomponent true "Field_LinearVelocity" null (`CullingField.SetCullingField` (`self.CullingField`) _returnvalue_2 (`RadialVector.SetRadialVector` (`self.RadialVector`) 1000.0 _returnvalue) "Field_Culling_Outside")))

(fn `UserConstructionScript`)